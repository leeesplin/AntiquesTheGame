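; Guide arrow actor that rotates relative to the player and current camera, and shows only when the player is off screen or far away.
; Each Tick, RotateArrow sets the mesh to the look-at rotation from the player to a point ahead of MainGameMode's CurrentCamera.
; ShowHideArrow hides the mesh while the player's head is on screen and within a distance threshold.
; The saved StartRotation feeds only unused nodes.
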(event `self.ReceiveBeginPlay`
  (set `self.StartRotation` (`SceneComponent.K2_GetComponentRotation` (`self.StaticMesh`))))

(event `self.ReceiveTick`
  (params (DeltaSeconds :type "Float (single-precision)"))
  (`self.RotateArrow`)
  (`self.ShowHideArrow`))

(fn `RotateArrow`
  (bind _asmain_game_mode (cast `/Game/Lee/MainGameMode` (`GameplayStatics.GetGameMode`)))
  (`/Engine/EditorBlueprintResources/StandardMacros.IsValid` (`/Game/Lee/MainGameMode.currentCamera` _asmain_game_mode)
    (:`Is Valid`
      (bind _asplayer_character (cast `/Game/Lee/PlayerCharacter` (`GameplayStatics.GetPlayerCharacter` 0)))
      (bind _asmain_game_mode_2 (cast `/Game/Lee/MainGameMode` (`GameplayStatics.GetGameMode`)))
      (bind _currentcamera (`/Game/Lee/MainGameMode.currentCamera` _asmain_game_mode_2))
      (`SceneComponent.K2_SetWorldRotation` (`self.StaticMesh`) (`KismetMathLibrary.FindLookAtRotation` (`self.K2_GetActorLocation` _asplayer_character) (+ (`SceneComponent.K2_GetComponentLocation` _currentcamera) (* (`SceneComponent.GetForwardVector` _currentcamera) 1000.0))) false false))))

(fn `ShowHideArrow`
  (bind _asplayer_character (cast `/Game/Lee/PlayerCharacter` (`GameplayStatics.GetPlayerCharacter` 0)))
  (if (`/Game/Lee/PlayerCharacter.isHeadOnScreen` _asplayer_character)
    (if (> (`/Game/Lee/PlayerCharacter.distanceFromCamera` _asplayer_character) 1000.0)
      (`SceneComponent.SetVisibility` (`self.StaticMesh`) true false :!label _label)
      (else
        (`SceneComponent.SetVisibility` (`self.StaticMesh`) false false)))
    (else
      (goto _label))))

(fn `UserConstructionScript`)