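; BP_NPC is an NPC that can wander between actors tagged "Waypoint".
; One second after BeginPlay, if ApplyGravity is set, it enables gravity and gathers those waypoints.
; If IsMovingAI is also set, it loops until the waypoint list is non-empty, then moves to a random entry with AIMoveTo.
; Each successful move picks another random waypoint, while failed moves have no handling.
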(event `self.ReceiveBeginPlay`
  (`KismetSystemLibrary.Delay` 1.0)
  (if (`self.applyGravity`)
    (`PrimitiveComponent.SetEnableGravity` (`self.CapsuleComponent`) true)
    (set `CharacterMovementComponent.GravityScale` 1.0 (`self.CharacterMovement`))
    (bind _outactors (`GameplayStatics.GetAllActorsWithTag` "Waypoint"))
    (set `self.waypoints` _outactors)
    (if (`self.isMovingAI`)
      (while (== (`KismetArrayLibrary.Array_Length` (`self.waypoints`)) 0)
        _)
      (bind _output_get (set `self.currentWaypoint` (`|GetArrayItem` (`self.waypoints`) (`KismetMathLibrary.RandomInteger` (`KismetArrayLibrary.Array_Length` (`self.waypoints`)))) :!label _label))
      (`|AIMoveTo` self (`self.K2_GetActorLocation` _output_get) _output_get
        (:`OnSuccess`
          (goto _label))))))

(event `self.ReceiveTick`
  (params (DeltaSeconds :type "Float (single-precision)")))

(fn `UserConstructionScript`)