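; BP_MusicController is an actor that plays a sequence of music tracks back to back.
; It starts the Music audio component on BeginPlay, then polls it every Tick.
; When playback stops, it increments MusicIterator, assigns that MusicArray entry if valid, and plays again.
; The index never wraps, so once it passes the array end, the last assigned sound keeps replaying.
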(event `self.ReceiveBeginPlay`
  (`AudioComponent.Play` (`self.Music`) 0.0))

(event `self.ReceiveTick`
  (params (DeltaSeconds :type "Float (single-precision)"))
  (if (not (`AudioComponent.IsPlaying` (`self.Music`)))
    (bind _result (`/Engine/EditorBlueprintResources/StandardMacros.IncrementInt` (`self.musicIterator`))
      (:`  `
        (bind _output (`|GetArrayItem` (`self.MusicArray`) _result))
        (`/Engine/EditorBlueprintResources/StandardMacros.IsValid` _output
          (:`Is Valid`
            (`AudioComponent.SetSound` (`self.Music`) _output))
          (:`Is Not Valid`
            _))
        (`AudioComponent.Play` (`self.Music`) 0.0)))))

(fn `UserConstructionScript`)